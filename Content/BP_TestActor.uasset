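; BP_TestActor is a test actor that exercises serial port communication from Blueprint.
; On BeginPlay it creates and opens a port on COM5 with a default config, writes a "0" string and prints the write result.
; Each Tick it polls the stored port while valid and prints any successfully read data to screen in green.
; The port is never explicitly closed.
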(event EventBeginPlay
  (bind _serialport (Class|Serial4UnrealBPLibrary|CreateSerialPort 5 (Utilities|Struct|MakePortConfig 9600 8)))
  (bind _output_get (Variables|Default|SetSerialPort _serialport))
  (Class|SerialPort|Open _output_get)
  (bind _returnvalue (Class|SerialPort|Write _output_get "0"))
  (Development|PrintString (Utilities|String|ToString(Integer) _returnvalue)))

(event EventTick
  (params (DeltaSeconds :type Float%20%28single-precision%29))
  (bind _serialport (Variables|Default|GetSerialPort))
  (Utilities|IsValid _serialport
    (:Is%20Valid
      (bind (_data _returnvalue) (Class|SerialPort|Read _serialport))
      (if _returnvalue
        (Development|PrintString _data true true "(R=0.000000,G=1.000000,B=0.000000,A=1.000000)")))))

(fn ConstructionScript)